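; BP_Bullet is a bullet actor that steps forward and knocks back the third-person character it hits.
; Each Shooting press prints a debug string and moves the actor along its forward vector by ShootSpeed in one unswept jump, with no continuous movement.
; Its Cube's hit event casts the other actor to BP_ThirdPersonCharacter and applies the negated NormalImpulse to its CharacterMovement.
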(event OnComponentHit(Cube)
  (params (HitComponent :type Primitive%20Component%20Object%20Reference) (OtherActor :type Actor%20Object%20Reference) (OtherComp :type Primitive%20Component%20Object%20Reference) (NormalImpulse :type Vector :default "0, 0, 0") (Hit :type Hit%20Result%20Structure%20%28by%20ref%29))
  ;[1 1 1] 총알에 맞을 시_플레이어가 뒤로 이동
  (bind _asbp_third_person_character (Utilities|Casting|CastToBP_ThirdPersonCharacter OtherActor))
  (Physics|AddImpulse (Variables|/Script/Engine.Character|GetCharacterMovement _asbp_third_person_character) (* NormalImpulse -1.0) false))

(event Input|ActionEvents|InputActionShooting
  (params (Key :type Key%20Structure :default "None"))
  (:Pressed
    (Development|PrintString "Shoot")
    (Transformation|SetActorLocation (+ (Transformation|GetActorLocation) (* (Transformation|GetActorForwardVector) (Variables|Default|GetShootSpeed))) false false)))

(fn ConstructionScript)