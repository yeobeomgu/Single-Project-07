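; BP_Town is an actor that periodically spawns BP_Fire actors at the world transform of its TownArrow component.
; Tick accumulates delta time into CurrentTime, then spawns and resets the timer once it reaches DelayTime.
; An unconnected graph fragment, which never runs, would randomly set Direction from the third-person character's rotation or the town's own eye view, weighted by TraceRate.
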(event EventTick
  (params (DeltaSeconds :type Float%20%28single-precision%29))
  (bind _output_get (Variables|Default|SetCurrentTime (+ DeltaSeconds (Variables|Default|GetCurrentTime))))
  (if (>= _output_get (Variables|Default|GetDelayTime))
    (Game|SpawnActorfromClass "/Game/BluePrint/BP_Fire.BP_Fire_C" (Transformation|GetWorldTransform (Variables|Default|GetTownArrow)) "Undefined" "MultiplyWithRoot" 0 0)
    (Variables|Default|SetCurrentTime 0.0)))

(event EventBeginPlay)

(fn ConstructionScript)