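; BP_MoveBox is a box actor that travels along a spline path once its Cube component registers a hit.
; On hit, it grabs a BP_Spline from the level via GetActorOfClass and plays a timeline at a rate set by Speed.
; The timeline's Move value maps to distance along the spline, setting location in world space and rotation in the spline's local space.
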(event OnComponentHit(Cube)
  (params (HitComponent :type Primitive%20Component%20Object%20Reference) (OtherActor :type Actor%20Object%20Reference) (OtherComp :type Primitive%20Component%20Object%20Reference) (NormalImpulse :type Vector :default "0, 0, 0") (Hit :type Hit%20Result%20Structure%20%28by%20ref%29))
  (bind _returnvalue (Actor|GetActorOfClass "/Game/BluePrint/BP_Spline.BP_Spline_C"))
  (Variables|Default|SetSpline_Select _returnvalue)
  (CallFunction|BoxMove))

(event Custom|BoxMove
  (Components|Timeline|SetPlayRate (Variables|Default|Get타임라인) (Variables|Default|GetSpeed))
  (bind _move (Timeline|타임라인 Play)
    (:Update
      (Transformation|SetActorTransform (Math|Transform|MakeTransform (Spline|GetLocationatDistanceAlongSpline (Variables|/Game/BluePrint/BP_Spline.BP_Spline_C|GetSpline (Variables|Default|GetSpline_select)) (Math|Float|Lerp 0.0 (Spline|GetSplineLength (Variables|/Game/BluePrint/BP_Spline.BP_Spline_C|GetSpline (Variables|Default|GetSpline_Select))) _move) "World") (Spline|GetRotationatDistanceAlongSpline (Variables|/Game/BluePrint/BP_Spline.BP_Spline_C|GetSpline (Variables|Default|GetSpline_Select)) (Math|Float|Lerp 0.0 (Spline|GetSplineLength (Variables|/Game/BluePrint/BP_Spline.BP_Spline_C|GetSpline (Variables|Default|GetSpline_Select))) _move) "Local") "1.000000,1.000000,1.000000")))))

(fn ConstructionScript)