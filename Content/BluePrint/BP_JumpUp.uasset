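; BP_JumpUp is a trigger actor that gives the third-person character a temporary jump boost.
; When the character overlaps its Box, it raises the movement component's JumpZVelocity by a large fixed amount and prints the new value on screen.
; After a one-second Delay it subtracts the same amount, and a threshold check on the current velocity keeps the boost from stacking.
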(event OnComponentBeginOverlap(Box)
  (params (OverlappedComponent :type Primitive%20Component%20Object%20Reference) (OtherActor :type Actor%20Object%20Reference) (OtherComp :type Primitive%20Component%20Object%20Reference) (OtherBodyIndex :type Integer) (bFromSweep :type Boolean) (SweepResult :type Hit%20Result%20Structure%20%28by%20ref%29))
  (bind _asbp_third_person_character (Utilities|Casting|CastToBP_ThirdPersonCharacter OtherActor))
  (if (< (Variables|/Script/Engine.CharacterMovementComponent|GetJumpZVelocity (Variables|/Script/Engine.Character|GetCharacterMovement _asbp_third_person_character)) 701.0)
    (bind _output_get (Variables|/Script/Engine.CharacterMovementComponent|SetJumpZVelocity (Variables|/Script/Engine.Character|GetCharacterMovement _asbp_third_person_character) (+ (Variables|/Script/Engine.CharacterMovementComponent|GetJumpZVelocity (Variables|/Script/Engine.Character|GetCharacterMovement _asbp_third_person_character)) 1e+03)))
    (Development|PrintString (Utilities|String|Append "점프력 700 -> 점프력 " (Utilities|String|ToString(Float) _output_get)))
    (Utilities|FlowControl|Delay 1.0)
    (Variables|/Script/Engine.CharacterMovementComponent|SetJumpZVelocity (Variables|/Script/Engine.Character|GetCharacterMovement _asbp_third_person_character) (- _output_get 1e+03))))

(fn ConstructionScript)