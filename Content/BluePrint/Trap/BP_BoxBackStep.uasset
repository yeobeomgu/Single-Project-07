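; Trap actor that shifts and tilts when something overlaps it.
; Any overlap on Box instantly moves Cube to a fixed relative offset along Y.
; When the player overlaps the actor below a height threshold, the whole actor rises and rolls, then reverses both changes after a three-second delay.
; Character impulse and explosion effect nodes exist but are never executed.
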(event OnComponentBeginOverlap(Box)
  (params (OverlappedComponent :type Primitive%20Component%20Object%20Reference) (OtherActor :type Actor%20Object%20Reference) (OtherComp :type Primitive%20Component%20Object%20Reference) (OtherBodyIndex :type Integer) (bFromSweep :type Boolean) (SweepResult :type Hit%20Result%20Structure%20%28by%20ref%29))
  (Transformation|SetRelativeLocation (Variables|Default|GetCube) "0.000000,400.000000,0.000000" false false)
  (bind _asbp_third_person_character (Utilities|Casting|CastToBP_ThirdPersonCharacter OtherActor)))

(event Collision|EventActorBeginOverlap
  (params (OtherActor :type Actor%20Object%20Reference))
  (bind _returnvalue (Transformation|GetActorRotation))
  (bind _returnvalue_2 (Transformation|GetActorLocation))
  (bind _returnvalue_3 (Transformation|GetActorLocation))
  (bind _returnvalue_4 (Transformation|GetActorRotation))
  (if (== OtherActor (Game|GetPlayerCharacter 0))
    (if (> 131.0 (.z (Transformation|GetActorLocation)))
      (Transformation|SetActorLocationAndRotation (Math|Vector|MakeVector (.x _returnvalue_2) (.y _returnvalue_2) (+ (.z _returnvalue_2) 5e+01)) (Math|Rotator|MakeRotator (+ (.roll _returnvalue) -3e+01) (.pitch _returnvalue) (.yaw _returnvalue)))
      (Utilities|FlowControl|Delay 3.0)
      (Transformation|SetActorLocationAndRotation (Math|Vector|MakeVector (.x _returnvalue_3) (.y _returnvalue_3) (- (.z _returnvalue_3) 5e+01)) (Math|Rotator|MakeRotator (+ (.roll _returnvalue_4) 3e+01) (.pitch _returnvalue_4) (.yaw _returnvalue_4))))))

(fn ConstructionScript)