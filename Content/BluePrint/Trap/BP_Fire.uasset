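; BP_Fire is a trap projectile that launches forward when it spawns and knocks back the player character on impact.
; BeginPlay applies a large physics impulse to its Cube along the actor's forward vector, then destroys the actor after five seconds.
; When the Cube hits a ThirdPerson character, it pushes the character's movement with a scaled-down hit impulse, spawns an explosion emitter and destroys itself.
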(event OnComponentHit(Cube)
  (params (HitComponent :type Primitive%20Component%20Object%20Reference) (OtherActor :type Actor%20Object%20Reference) (OtherComp :type Primitive%20Component%20Object%20Reference) (NormalImpulse :type Vector :default "0, 0, 0") (Hit :type Hit%20Result%20Structure%20%28by%20ref%29))
  (bind _asbp_third_person_character (Utilities|Casting|CastToBP_ThirdPersonCharacter OtherActor))
  (Physics|AddImpulse (Variables|/Script/Engine.Character|GetCharacterMovement _asbp_third_person_character) (* NormalImpulse 0.03) false)
  (Development|PrintString "맞음")
  (Effects|SpawnEmitteratLocation "/Game/StarterContent/Particles/P_Explosion.P_Explosion" (Class|CharacterMovementComponent|GetLastUpdateLocation (Variables|/Script/Engine.Character|GetCharacterMovement _asbp_third_person_character)))
  (Actor|DestroyActor))

(event EventBeginPlay
  (Physics|AddImpulse (Variables|Default|GetCube) (* (Transformation|GetActorForwardVector) 2e+06) "None" false)
  (Utilities|FlowControl|Delay 5.0)
  (Actor|DestroyActor))

(fn ConstructionScript)