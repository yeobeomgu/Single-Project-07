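; BP_Town is a turret-style trap that turns to face the player and periodically fires BP_Fire actors.
; Each Tick, while player character 0 is valid, it rotates its root toward the player using RInterpToConstant at InterpSpeed.
; It also accumulates DeltaSeconds in CurrentTime, spawning BP_Fire at the TownArrow transform and resetting the timer whenever DelayTime is reached.
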(event EventTick
  (params (DeltaSeconds :type Float%20%28single-precision%29))
  (bind _returnvalue (Game|GetPlayerCharacter 0))
  (bind _defaultsceneroot (Variables|Default|GetDefaultSceneRoot))
  (bind _interp_speed (Variables|Default|GetInterp%20Speed))
  (bind _defaultsceneroot_2 (Variables|Default|GetDefaultSceneRoot))
  (bind _returnvalue_2 (Transformation|GetWorldLocation _defaultsceneroot))
  (bind _returnvalue_3 (Transformation|GetWorldRotation _defaultsceneroot_2))
  (bind _rootcomponent (Variables|/Script/Engine.Actor|GetRootComponent _returnvalue))
  (bind _returnvalue_4 (Transformation|GetWorldLocation _rootcomponent))
  (bind _returnvalue_5 (Math|Rotator|FindLookatRotation _returnvalue_2 (Math|Vector|MakeVector (.x _returnvalue_4) (.y _returnvalue_4) (.z _returnvalue_4))))
  (bind _returnvalue_6 (Class|KismetMathLibrary|RInterptoConstant _returnvalue_3 _returnvalue_5 DeltaSeconds _interp_speed))
  (if true
    (Utilities|IsValid _returnvalue
      (:Is%20Valid
        (Transformation|SetWorldRotation (Variables|Default|GetDefaultSceneRoot) (Math|Rotator|MakeRotator (.roll _returnvalue_6) (.pitch _returnvalue_6) (.yaw _returnvalue_6)) false false)
        (bind _output_get (Variables|Default|SetCurrentTime (+ DeltaSeconds (Variables|Default|GetCurrentTime))))
        (if (>= _output_get (Variables|Default|GetDelayTime))
          (Game|SpawnActorfromClass "/Game/BluePrint/Trap/BP_Fire.BP_Fire_C" (Transformation|GetWorldTransform (Variables|Default|GetTownArrow)) "Undefined" "MultiplyWithRoot" 0 0)
          (Variables|Default|SetCurrentTime 0.0))))))

(fn ConstructionScript)