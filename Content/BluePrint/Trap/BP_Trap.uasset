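; BP_Trap is a moving hazard whose Cube slides back and forth along relative X between roughly 0 and 300.
; Tick drives the motion with a fixed per-frame step and a direction flag, so speed depends on frame rate.
; When the third-person character overlaps the Cube, it adds damage and gauge through BP_PlayerState, spawns an explosion and shifts the character along negative Y.
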(event OnComponentBeginOverlap(Cube)
  (params (OverlappedComponent :type Primitive%20Component%20Object%20Reference) (OtherActor :type Actor%20Object%20Reference) (OtherComp :type Primitive%20Component%20Object%20Reference) (OtherBodyIndex :type Integer) (bFromSweep :type Boolean) (SweepResult :type Hit%20Result%20Structure%20%28by%20ref%29))
  ;[1 1 1] 플레이어 닿음
  (bind _asbp_third_person_character (Utilities|Casting|CastToBP_ThirdPersonCharacter OtherActor))
  (bind _asbp_player_state (Utilities|Casting|CastToBP_PlayerState (Variables|/Script/Engine.Pawn|GetPlayerState _asbp_third_person_character)))
  (Default|AddDamage _asbp_player_state 0.5)
  (Default|AddGauge _asbp_player_state 1.0)
  (Effects|SpawnEmitteratLocation "/Game/StarterContent/Particles/P_Explosion.P_Explosion" (Transformation|GetActorLocation _asbp_third_person_character))
  (Transformation|SetRelativeLocation (Variables|/Script/Engine.Actor|GetRootComponent _asbp_third_person_character) (+ (Transformation|GetActorLocation _asbp_third_person_character) "0.000000,-20.000000,0.000000") false false))

(event EventTick
  (params (DeltaSeconds :type Float%20%28single-precision%29))
  ;[1 1 1] 이동한다.
  (if (Variables|Default|GetBool)
    (Variables|Default|SetVertical (+ (Variables|Default|GetVertical) 2.0))
    (Transformation|SetRelativeLocation (Variables|Default|GetCube) (Math|Vector|MakeVector (Variables|Default|GetVertical) 0.0 0.0) false false)
    (if (> (Variables|Default|GetVertical) 3e+02)
      (Variables|Default|SetBool false))
    (else
      (Variables|Default|SetVertical (- (Variables|Default|GetVertical) 2.0))
      (Transformation|SetRelativeLocation (Variables|Default|GetCube) (Math|Vector|MakeVector (Variables|Default|GetVertical) 0.0 0.0) false false)
      (if (< (Variables|Default|GetVertical) 0.0)
        (Variables|Default|SetBool true)))))

(fn ConstructionScript)