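; BP_RotationCyilnder is a trap actor whose Cube component rolls back and forth.
; Each Tick steps a Time counter up or down according to the GoStop flag and applies it as the Cube's relative roll, with pitch and yaw held at zero.
; GoStop flips when the counter passes either end of its range.
; The step ignores delta time, so rotation speed depends on frame rate.
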(event EventTick
  (params (DeltaSeconds :type Float%20%28single-precision%29))
  (if (Variables|Default|GetGoStop)
    (Variables|Default|SetTime (+ (Variables|Default|GetTime) 1.0))
    (Transformation|SetRelativeRotation (Variables|Default|GetCube) (Math|Rotator|MakeRotator (Variables|Default|GetTime) 0.0 0.0) false false)
    (if (> (Variables|Default|GetTime) 3e+02)
      (Variables|Default|SetGoStop false))
    (else
      (Variables|Default|SetTime (+ (Variables|Default|GetTime) -1.0))
      (Transformation|SetRelativeRotation (Variables|Default|GetCube) (Math|Rotator|MakeRotator (Variables|Default|GetTime) 0.0 0.0) false false)
      (if (< (Variables|Default|GetTime) 0.0)
        (Variables|Default|SetGoStop true)))))

(fn ConstructionScript)