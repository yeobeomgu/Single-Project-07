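; BP_Water is a water trap that hurts the player character on contact.
; When the Water component is overlapped by a BP_ThirdPersonCharacter, it adds damage and gauge to that character's BP_PlayerState.
; It then sets the character slightly above its movement component's last update location and spawns an explosion particle effect below that location.
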(event OnComponentBeginOverlap(Water)
  (params (OverlappedComponent :type Primitive%20Component%20Object%20Reference) (OtherActor :type Actor%20Object%20Reference) (OtherComp :type Primitive%20Component%20Object%20Reference) (OtherBodyIndex :type Integer) (bFromSweep :type Boolean) (SweepResult :type Hit%20Result%20Structure%20%28by%20ref%29))
  (bind _asbp_third_person_character (Utilities|Casting|CastToBP_ThirdPersonCharacter OtherActor))
  (bind _asbp_player_state (Utilities|Casting|CastToBP_PlayerState (Variables|/Script/Engine.Pawn|GetPlayerState _asbp_third_person_character)))
  (Default|AddDamage _asbp_player_state 0.5)
  (Default|AddGauge _asbp_player_state 1.0)
  (Transformation|SetActorLocation _asbp_third_person_character (Math|Vector|MakeVector (.x (Class|CharacterMovementComponent|GetLastUpdateLocation (Variables|/Script/Engine.Character|GetCharacterMovement _asbp_third_person_character))) (.y (Class|CharacterMovementComponent|GetLastUpdateLocation (Variables|/Script/Engine.Character|GetCharacterMovement _asbp_third_person_character))) (+ (.z (Class|CharacterMovementComponent|GetLastUpdateLocation (Variables|/Script/Engine.Character|GetCharacterMovement _asbp_third_person_character))) 5.0)) false false)
  (Effects|SpawnEmitteratLocation "/Game/StarterContent/Particles/P_Explosion.P_Explosion" (Math|Vector|MakeVector (.x (Class|CharacterMovementComponent|GetLastUpdateLocation (Variables|/Script/Engine.Character|GetCharacterMovement _asbp_third_person_character))) (.y (Class|CharacterMovementComponent|GetLastUpdateLocation (Variables|/Script/Engine.Character|GetCharacterMovement _asbp_third_person_character))) (+ (.z (Class|CharacterMovementComponent|GetLastUpdateLocation (Variables|/Script/Engine.Character|GetCharacterMovement _asbp_third_person_character))) -1e+02))))

(fn ConstructionScript)